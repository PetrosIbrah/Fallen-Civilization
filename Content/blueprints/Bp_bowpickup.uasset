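; Bow pickup actor that the player collects by pressing E while standing inside its sphere.
; Sphere overlaps with Bp_player enable input on the actor and disable it when the overlap ends.
; Pressing E casts the overlapping actor to Bp_player, passes the SM_Bow_01 component or mesh to its Bowpickup function, then destroys the pickup and plays an equip sound.
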(event `Key|E`
  (params (Key :type "Key Structure"))
  (:`Pressed`
    (bind _asbp_player (cast `/Game/blueprints/Bp_player` (stale `self.Sphere.OnComponentBeginOverlap` OtherActor)))
    (`/Game/blueprints/Bp_player.bowpickup` _asbp_player "/Game/LP_RPGWeapons_JC/Models/SM_Bow_01.SM_Bow_01")
    (`self.K2_DestroyActor`)
    (`GameplayStatics.PlaySound2D` "/Game/sounds/Equip.Equip" 1.0 1.0 0.0 null null)))

(event `self.Sphere.OnComponentBeginOverlap`
  (params (OverlappedComponent :type "PrimitiveComponent Object Reference") (OtherActor :type "Actor Object Reference") (OtherComp :type "PrimitiveComponent Object Reference") (OtherBodyIndex :type Integer) (bFromSweep :type Boolean) (SweepResult :type "HitResult Structure (by ref)"))
  (cast `/Game/blueprints/Bp_player` OtherActor)
  (`self.EnableInput` (`GameplayStatics.GetPlayerController` 0)))

(event `self.Sphere.OnComponentEndOverlap`
  (params (OverlappedComponent :type "PrimitiveComponent Object Reference") (OtherActor :type "Actor Object Reference") (OtherComp :type "PrimitiveComponent Object Reference") (OtherBodyIndex :type Integer))
  (cast `/Game/blueprints/Bp_player` OtherActor)
  (`self.DisableInput` (`GameplayStatics.GetPlayerController` 0)))

(fn `UserConstructionScript`)