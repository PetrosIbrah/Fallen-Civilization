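; Player character that moves, looks and jumps through Enhanced Input, talks to NPCs and wears picked-up gear.
; BeginPlay adds the input mapping context and puts the coin and help-sign widgets on screen.
; Five duplicate E-key handlers, one per NPC class, send TalkMessage to overlapping actors implementing the Bp_dialogue interface.
; Equip events set helmet, sword, bow or shield meshes and snap them to mesh sockets.
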(event `self.ReceiveBeginPlay`
  (`|ExecutionSequence`
    (:`then_0`
      (bind _asplayer_controller (cast `PlayerController` (`GameplayStatics.GetPlayerController` 0)))
      (bind _returnvalue (pcsubsystem `EnhancedInputLocalPlayerSubsystem` _asplayer_controller))
      (`/Engine/EditorBlueprintResources/StandardMacros.IsValid` _returnvalue
        (:`Is Valid`
          (`EnhancedInputSubsystemInterface.AddMappingContext` _returnvalue "/Game/imput/IMC_Playerimput.IMC_Playerimput" 0 (struct)))))
    (:`then_1`
      (bind _returnvalue_2 (`|CreateWidget` "/Game/Shop/Coin/WP_Coin.WP_Coin_C"))
      (`UserWidget.AddToViewport` _returnvalue_2 0))
    (:`then_2`
      (bind _returnvalue_3 (`|CreateWidget` "/Game/Online_Help/WP_HelpSign.WP_HelpSign_C"))
      (`UserWidget.AddToViewport` _returnvalue_3 0))))

(event `EnhancedInput|/Game/imput/IA_Jump`
  (params (ActionValue :type Boolean) (ElapsedSeconds :type "Float (double-precision)") (TriggeredSeconds :type "Float (double-precision)") (InputAction :type "InputAction Object Reference" :default "/Game/imput/IA_Jump.IA_Jump"))
  (:`Started`
    (`self.Jump`))
  (:`Canceled`
    (`self.StopJumping` :!label _label))
  (:`Completed`
    (goto _label)))

(event `EnhancedInput|/Game/imput/IA_move`
  (params (ActionValue :type "Vector2D Structure") (ElapsedSeconds :type "Float (double-precision)") (TriggeredSeconds :type "Float (double-precision)") (InputAction :type "InputAction Object Reference" :default "/Game/imput/IA_move.IA_move"))
  (bind (_returnvalue_roll _returnvalue_pitch _returnvalue_yaw) (`KismetMathLibrary.BreakRotator` (`self.GetControlRotation`)))
  (bind (_returnvalue_roll_2 _returnvalue_pitch_2 _returnvalue_yaw_2) (`KismetMathLibrary.BreakRotator` (`self.GetControlRotation`)))
  (:`Triggered`
    (`self.AddMovementInput` (`KismetMathLibrary.GetRightVector` (`KismetMathLibrary.MakeRotator` _returnvalue_roll_2 0.0 _returnvalue_yaw_2)) ActionValue_X)
    (`self.AddMovementInput` (`KismetMathLibrary.GetForwardVector` (`KismetMathLibrary.MakeRotator` _returnvalue_roll 0.0 _returnvalue_yaw)) ActionValue_Y)))

(event `Key|E`
  (params (Key :type "Key Structure"))
  (:`Pressed`
    (for _array_element (`self.GetOverlappingActors` "/Game/NPCs/king_npc/pb_npccharacter.pb_npccharacter_C")
      (if (`KismetSystemLibrary.DoesImplementInterface` _array_element "/Game/NPCs/knight_npc/bp_dialogue.bp_dialogue_C")
        (message `/Game/NPCs/knight_npc/bp_dialogue.Talk` _array_element)))))

(event `EnhancedInput|/Game/imput/IA_Look`
  (params (ActionValue :type "Vector2D Structure") (ElapsedSeconds :type "Float (double-precision)") (TriggeredSeconds :type "Float (double-precision)") (InputAction :type "InputAction Object Reference" :default "/Game/imput/IA_Look.IA_Look"))
  (:`Triggered`
    (`self.AddControllerYawInput` ActionValue_X)
    (`self.AddControllerPitchInput` (* ActionValue_Y -1.0))))

(event `Key|E`
  (params (Key :type "Key Structure"))
  (:`Pressed`
    (for _array_element (`self.GetOverlappingActors` "/Game/NPCs/shop_npc/pb_npccharacter1.pb_npccharacter1_C")
      (if (`KismetSystemLibrary.DoesImplementInterface` _array_element "/Game/NPCs/knight_npc/bp_dialogue.bp_dialogue_C")
        (message `/Game/NPCs/knight_npc/bp_dialogue.Talk` _array_element)))))

(event `Equiphalmet`
  (params (NewMesh :type "StaticMesh Object Reference"))
  (`StaticMeshComponent.SetStaticMesh` (`self.helmentmesh`) NewMesh)
  (`SceneComponent.K2_AttachToComponent` (`self.helmentmesh`) (`self.Mesh`) "helmetSocket" "SnapToTarget" "SnapToTarget" "SnapToTarget" true))

(event `Key|E`
  (params (Key :type "Key Structure"))
  (:`Pressed`
    (for _array_element (`self.GetOverlappingActors` "/Game/NPCs/farmer_npc/pb_npccharacter2.pb_npccharacter2_C")
      (if (`KismetSystemLibrary.DoesImplementInterface` _array_element "/Game/NPCs/knight_npc/bp_dialogue.bp_dialogue_C")
        (message `/Game/NPCs/knight_npc/bp_dialogue.Talk` _array_element)))))

(event `Key|E`
  (params (Key :type "Key Structure"))
  (:`Pressed`
    (for _array_element (`self.GetOverlappingActors` "/Game/NPCs/instructor_npc/pb_npccharacter3.pb_npccharacter3_C")
      (if (`KismetSystemLibrary.DoesImplementInterface` _array_element "/Game/NPCs/knight_npc/bp_dialogue.bp_dialogue_C")
        (message `/Game/NPCs/knight_npc/bp_dialogue.Talk` _array_element)))))

(event `equipsword`
  (params (NewMesh :type "StaticMesh Object Reference"))
  (`StaticMeshComponent.SetStaticMesh` (`self.swordmesh`) NewMesh)
  (`SceneComponent.K2_AttachToComponent` (`self.swordmesh`) (`self.Mesh`) "swordsocket" "SnapToTarget" "SnapToTarget" "SnapToTarget" true))

(event `Key|E`
  (params (Key :type "Key Structure"))
  (:`Pressed`
    (for _array_element (`self.GetOverlappingActors` "/Game/NPCs/knight_npc/pb_npccharacter4.pb_npccharacter4_C")
      (if (`KismetSystemLibrary.DoesImplementInterface` _array_element "/Game/NPCs/knight_npc/bp_dialogue.bp_dialogue_C")
        (message `/Game/NPCs/knight_npc/bp_dialogue.Talk` _array_element)))))

(event `bowpickup`
  (params (NewMesh :type "StaticMesh Object Reference"))
  (`StaticMeshComponent.SetStaticMesh` (`self.bowmesh`) NewMesh)
  (`SceneComponent.K2_AttachToComponent` (`self.bowmesh`) (`self.Mesh`) "bowshocket" "SnapToTarget" "SnapToTarget" "SnapToTarget" true))

(event `shielldpickup`
  (params (NewMesh :type "StaticMesh Object Reference"))
  (`StaticMeshComponent.SetStaticMesh` (`self.shieldmesh`) NewMesh)
  (`SceneComponent.K2_AttachToComponent` (`self.shieldmesh`) (`self.Mesh`) "shieldsocket" "SnapToTarget" "SnapToTarget" "SnapToTarget" true))

(fn `UserConstructionScript`)