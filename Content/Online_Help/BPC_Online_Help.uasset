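; Component that toggles an online help widget on screen with the H key.
; BeginPlay creates the WP_Online_Help widget once and keeps it for reuse.
; Pressing H adds or removes it from the viewport based on visibility, switching the player 0 mouse cursor and input mode between Game And UI and Game Only.
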(event `self.ReceiveBeginPlay`
  (bind _returnvalue (`|CreateWidget` "/Game/Online_Help/UI/WP_Online_Help.WP_Online_Help_C"))
  (set `self.Online_Help` _returnvalue))

(event `Key|H`
  (params (Key :type "Key Structure"))
  (bind _returnvalue (`GameplayStatics.GetPlayerController` 0))
  (bind _returnvalue_2 (`GameplayStatics.GetPlayerController` 0))
  (bind _online_help (`self.Online_Help`))
  (:`Pressed`
    (if (`Widget.IsVisible` (`self.Online_Help`))
      (`Widget.RemoveFromParent` _online_help)
      (set `PlayerController.bShowMouseCursor` false _returnvalue_2)
      (`WidgetBlueprintLibrary.SetInputMode_GameOnly` _returnvalue_2)
      (else
        (set `PlayerController.bShowMouseCursor` true _returnvalue)
        (`WidgetBlueprintLibrary.SetInputMode_GameAndUIEx` _returnvalue null)
        (`UserWidget.AddToViewport` _online_help 0)))))