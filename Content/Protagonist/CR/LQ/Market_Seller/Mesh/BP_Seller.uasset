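; BP_Seller is a market seller actor that opens a shop UI when the player comes close.
; Entering its Sphere as Bp_player creates the WP_Shop widget, shows the mouse cursor and switches input to Game and UI.
; Leaving the sphere removes top-level widgets found by class lookup, hides the cursor and restores game-only input.
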(event `self.Sphere.OnComponentBeginOverlap`
  (params (OverlappedComponent :type "PrimitiveComponent Object Reference") (OtherActor :type "Actor Object Reference") (OtherComp :type "PrimitiveComponent Object Reference") (OtherBodyIndex :type Integer) (bFromSweep :type Boolean) (SweepResult :type "HitResult Structure (by ref)"))
  (bind _returnvalue (`GameplayStatics.GetPlayerController` 0))
  (cast `/Game/blueprints/Bp_player` OtherActor)
  (bind _returnvalue_2 (`|CreateWidget` "/Game/Shop/Coin/WP_Shop.WP_Shop_C"))
  (`UserWidget.AddToViewport` _returnvalue_2 0)
  (set `PlayerController.bShowMouseCursor` true _returnvalue)
  (`WidgetBlueprintLibrary.SetInputMode_GameAndUIEx` _returnvalue null))

(event `self.Sphere.OnComponentEndOverlap`
  (params (OverlappedComponent :type "PrimitiveComponent Object Reference") (OtherActor :type "Actor Object Reference") (OtherComp :type "PrimitiveComponent Object Reference") (OtherBodyIndex :type Integer))
  (bind _returnvalue (`GameplayStatics.GetPlayerController` 0))
  (cast `/Game/blueprints/Bp_player` OtherActor)
  (bind _foundwidgets (`WidgetBlueprintLibrary.GetAllWidgetsOfClass` (`self.Widget Class`)))
  (`Widget.RemoveFromParent` _foundwidgets)
  (set `PlayerController.bShowMouseCursor` false _returnvalue)
  (`WidgetBlueprintLibrary.SetInputMode_GameOnly` _returnvalue))

(fn `UserConstructionScript`)